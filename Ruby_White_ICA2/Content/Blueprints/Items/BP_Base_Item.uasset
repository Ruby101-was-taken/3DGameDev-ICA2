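; BP_Base_Item is a base item actor that players can inspect.
; Its construction script applies the configured scale and inspection rotation to its mesh.
; Inspect, when the item is flagged inspectable, spawns a BP_InspectItem far from the world origin and passes it the player, static mesh, name and description, then returns it.
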(fn `Inspect`
  (params (player :type "/Game/Blueprints/Player/BP_FirstPersonCharacter Object Reference"))
  (returns (item :type "/Game/Blueprints/Inspection/Items/BP_InspectItem Object Reference"))
  (if (`self.is_inspectable`)
    (bind _returnvalue (`|SpawnActorFromClass` "/Game/Blueprints/Inspection/Items/BP_InspectItem.BP_InspectItem_C" (`KismetMathLibrary.MakeTransform` (10000000.0 0.0 0.0)) "Undefined" "MultiplyWithRoot" null null))
    (`/Game/Blueprints/Inspection/Items/BP_InspectItem.Inspect ` _returnvalue player (`StaticMeshComponent.StaticMesh` (`self.Mesh`)) (`self.item_name`) (`self.item_desc`))
    (return _returnvalue)))

(fn `UserConstructionScript`
  (bind _mesh (`self.Mesh`))
  (`|ExecutionSequence`
    (:`then_0`
      (`SceneComponent.SetRelativeScale3D` _mesh (`self.item_scale`)))
    (:`then_1`
      (`SceneComponent.K2_SetRelativeRotation` _mesh (`self.item_inspection_rotation`) false false))))