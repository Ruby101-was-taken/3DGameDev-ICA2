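; BP_InspectItem is an inspection actor that displays a given item for the player to rotate and zoom.
; Inspect sets the mesh, shows a W_Inspect widget with name and description, and disables character movement.
; Rotation is split between clamped pitch on the Empty component and free yaw on the mesh, while zoom adjusts a clamped SceneCaptureComponent2D FOV.
; Hide removes the widget and destroys the actor without restoring movement itself.
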(event `/Game/Blueprints/Inspection/Interface/BPI_Interactable.Inspect `
  (params (character :type "/Game/Blueprints/Player/BP_FirstPersonCharacter Object Reference") (inspected_item :type "StaticMesh Object Reference") (item_name :type Text) (item_desc :type Text))
  (`StaticMeshComponent.SetStaticMesh` (`self.Mesh`) inspected_item)
  (bind _returnvalue (`|CreateWidget` "/Game/UI/Inspect/W_Inspect.W_Inspect_C" null item_name item_desc))
  (`UserWidget.AddToViewport` _returnvalue 0)
  (set `/Game/Blueprints/Player/BP_FirstPersonCharacter.can_move` false character)
  (set `self.UI` _returnvalue))

(fn `Hide`
  (`Widget.RemoveFromParent` (`self.UI`))
  (`self.K2_DestroyActor`))

(fn `Rotate_Hor`
  (params (by :type "Float (double-precision)"))
  (`SceneComponent.K2_AddRelativeRotation` (`self.Empty`) (`KismetMathLibrary.MakeRotator` 0.0 (* by -1.0)) false false)
  (`SceneComponent.K2_SetRelativeRotation` (`self.Empty`) (`KismetMathLibrary.MakeRotator` 0.0 (`KismetMathLibrary.FMin` (`KismetMathLibrary.FMax` (.pitch (.rotation (`SceneComponent.GetRelativeTransform` (`self.Empty`)))) -80.0) 80.0)) false false))

(fn `Rotate_Ver`
  (params (by :type "Float (double-precision)"))
  (`SceneComponent.K2_AddRelativeRotation` (`self.Mesh`) (`KismetMathLibrary.MakeRotator` 0.0 0.0 by) false false)
  (return))

(fn `UserConstructionScript`)

(fn `Zoom`
  (params (zoom :type "Float (double-precision)"))
  (bind _scenecapturecomponent2d (`self.SceneCaptureComponent2D`))
  (set `SceneCaptureComponent2D.FOVAngle` (`KismetMathLibrary.FMin` (`KismetMathLibrary.FMax` (- (`SceneCaptureComponent2D.FOVAngle` _scenecapturecomponent2d) zoom) 15.0) 50.0) _scenecapturecomponent2d))