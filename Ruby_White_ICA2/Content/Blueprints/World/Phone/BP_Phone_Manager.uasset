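; Phone manager Blueprint that builds a dialed number from keypad input and plays the audio clip mapped to it.
; AddDigit appends digits, treats -1 as backspace and other negatives as submit, then updates a text render display.
; Submitting locks all level-gathered BP_Phone_Button actors and looks up the number as a Sounds data table row.
; The keypad unlocks after the clip plus a short delay, or immediately if no row matches.
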(event `self.ReceiveBeginPlay`
  (bind _outactors (`GameplayStatics.GetAllActorsOfClass` "/Game/Blueprints/World/Phone/BP_Phone_Button.BP_Phone_Button_C"))
  (set `self.keypad` _outactors))

(event `PlayPhoneAudio`
  (params (sound :type "SoundWave Object Reference"))
  (`GameplayStatics.PlaySound2D` sound 1.0 1.0 0.0 null null)
  (`KismetSystemLibrary.Delay` (`SoundBase.Duration` sound))
  (`KismetSystemLibrary.Delay` 1.0)
  (`self.SetKeypadLockStatus` false))

(fn `AddDigit`
  (params (digit :type Integer))
  (bind _full_number (`self.full_number`))
  (bind _full_number_2 (`self.full_number`))
  (if (>= digit 0)
    ; Simple Digit
    (set `self.full_number` (`KismetStringLibrary.Concat_StrStr` (`self.full_number`) (`KismetStringLibrary.Conv_IntToString` digit)))
    (elif (== digit -1)
      ; Remove Digit
      (set `self.full_number` (`KismetStringLibrary.GetSubstring` _full_number 0 (- (`KismetStringLibrary.Len` _full_number) 1)))
      (else
        (`self.SubmitNumber`))))
  (`TextRenderComponent.K2_SetText` (`self.TextRender`) (`KismetMathLibrary.SelectText` (`KismetTextLibrary.Conv_StringToText` _full_number_2) "..." (> (`KismetStringLibrary.Len` _full_number_2) 0))))

(fn `SetKeypadLockStatus`
  (params (is_Locked :type Boolean))
  (for _array_element (`self.keypad`)
    (`/Game/Blueprints/World/Phone/BP_Phone_Button.SetLockStatus` _array_element is_Locked)))

(fn `SubmitNumber`
  (`self.SetKeypadLockStatus` true)
  (bind _returnvalue (`|GetDataTableRow` (`self.sounds`) (`KismetStringLibrary.Conv_StringToName` (`self.full_number`)))
    (:`then`
      (`self.PlayPhoneAudio` (`.audio_clip_5_CE8C2B594CC29D80798C80AD4D2F6C36` (break `/Game/Blueprints/Structs/Phone/S_Phone_Number` _returnvalue))))
    (:`RowNotFound`
      (`self.SetKeypadLockStatus` false)))
  (set `self.full_number` ""))

(fn `UserConstructionScript`)