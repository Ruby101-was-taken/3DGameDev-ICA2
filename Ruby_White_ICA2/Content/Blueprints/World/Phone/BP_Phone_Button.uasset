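; BP_Phone_Button is a single key on an in-world phone, labeled with a digit or an arrow for negative special values.
; The construction script sets its text label from the Digit value.
; Push locks the button and sends Digit to the BP_Phone_Manager found at BeginPlay.
; Tick then drives a sine-based, frame-by-frame press offset until a timer expires, resetting the button's position and re-enabling it.
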(event `self.ReceiveBeginPlay`
  (bind _returnvalue (`GameplayStatics.GetActorOfClass` "/Game/Blueprints/World/Phone/BP_Phone_Manager.BP_Phone_Manager_C"))
  (set `self.phone_manager` _returnvalue))

(event `self.ReceiveTick`
  (params (DeltaSeconds :type "Float (single-precision)"))
  (if (`self.is_being_pushed`)
    (bind _output_get (set `self.pushed_timer` (+ (`self.pushed_timer`) (* DeltaSeconds (`self.push_speed`)))))
    (`SceneComponent.K2_AddLocalOffset` (`self.Button`) (`KismetMathLibrary.MakeVector` (* (`KismetMathLibrary.Sin` _output_get) -1.0)) false false)
    (if (>= (`self.pushed_timer`) 2.0)
      (set `self.can_be_pushed` true)
      (set `self.is_being_pushed` false)
      (`SceneComponent.K2_SetRelativeLocation` (`self.Button`) (0.0 0.0 0.0) false false))))

(fn `GetButtonText`
  (returns (text :type Text))
  (if (>= (`self.digit`) 0)
    (return (`KismetTextLibrary.Conv_IntToText` (`self.digit`)))
    (elif (== (`self.digit`) -1)
      (return "<-")
      (elif (== (`self.digit`) -10)
        (return "->")))))

(fn `Push`
  (if (`self.can_be_pushed`)
    (set `self.can_be_pushed` false)
    (set `self.is_being_pushed` true)
    (set `self.pushed_timer` 0.0)
    (`/Game/Blueprints/World/Phone/BP_Phone_Manager.AddDigit` (`self.phone_manager`) (`self.digit`))))

(fn `UserConstructionScript`
  (`TextRenderComponent.K2_SetText` (`self.TextRender`) (`self.GetButtonText`)))