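; BP_Phone_Button is a numbered phone button actor that animates a press when pushed.
; The construction script writes its Number onto a text render.
; Push clears CanBePushed and restarts a timer that Tick advances by PushSpeed, nudging the button along local X by a negative sine offset each frame.
; When the timer reaches its limit, the button snaps to its reset location and becomes pushable again.
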(event `self.ReceiveTick`
  (params (DeltaSeconds :type "Float (single-precision)"))
  (if (`self.is_being_pushed`)
    (bind _output_get (set `self.pushed_timer` (+ (`self.pushed_timer`) (* DeltaSeconds (`self.push_speed`)))))
    (`SceneComponent.K2_AddLocalOffset` (`self.Button`) (`KismetMathLibrary.MakeVector` (* (`KismetMathLibrary.Sin` _output_get) -1.0)) false false)
    (if (>= (`self.pushed_timer`) 2.0)
      (set `self.can_be_pushed` true)
      (set `self.is_being_pushed` false)
      (`SceneComponent.K2_SetRelativeLocation` (`self.Button`) (0.0 0.0 0.0) false false))))

(fn `Push`
  (set `self.can_be_pushed` false)
  (set `self.is_being_pushed` true)
  (set `self.pushed_timer` 0.0))

(fn `UserConstructionScript`
  (`TextRenderComponent.K2_SetText` (`self.TextRender`) (`KismetTextLibrary.Conv_IntToText` (`self.number`))))